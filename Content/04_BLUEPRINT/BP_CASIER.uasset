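; BP_CASIER is a locker actor whose door swings open when the first-person character approaches and closes when they leave.
; The Construction Script rebuilds the body from hard-coded instances on an instanced static mesh.
; Sphere overlap events restart separate opening and closing timelines that lerp the door pivot's yaw through a quarter turn.
; BeginPlay disables collision on the body, door and Cube1.
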(event `self.ReceiveBeginPlay`
  (`PrimitiveComponent.SetCollisionEnabled` (`self.CorpsCasier_ISM`) "NoCollision")
  (`PrimitiveComponent.SetCollisionEnabled` (`self.Porte`) "NoCollision")
  (`PrimitiveComponent.SetCollisionEnabled` (`self.Cube1`) "NoCollision"))

(event `self.sphere collision.OnComponentBeginOverlap`
  (params (OverlappedComponent :type "PrimitiveComponent Object Reference") (OtherActor :type "Actor Object Reference") (OtherComp :type "PrimitiveComponent Object Reference") (OtherBodyIndex :type Integer) (bFromSweep :type Boolean) (SweepResult :type "HitResult Structure (by ref)"))
  (cast `/Game/FirstPerson/Blueprints/BP_FirstPersonCharacter` OtherActor)
  (bind (_direction _newtrack_0) (`Timeline|Timeline` :!via `PlayFromStart`)
    (:`Update`
      (`SceneComponent.K2_SetRelativeRotation` (`self.Pivot porte`) (`KismetMathLibrary.MakeRotator` 0.0 0.0 (`KismetMathLibrary.Lerp` 0.0 -90.0 _newtrack_0)) false false))))

(event `self.sphere collision.OnComponentEndOverlap`
  (params (OverlappedComponent :type "PrimitiveComponent Object Reference") (OtherActor :type "Actor Object Reference") (OtherComp :type "PrimitiveComponent Object Reference") (OtherBodyIndex :type Integer))
  (cast `/Game/FirstPerson/Blueprints/BP_FirstPersonCharacter` OtherActor)
  (bind (_direction _newtrack_0) (`Timeline|Timeline_0` :!via `PlayFromStart`)
    (:`Update`
      (`SceneComponent.K2_SetRelativeRotation` (`self.Pivot porte`) (`KismetMathLibrary.MakeRotator` 0.0 0.0 (`KismetMathLibrary.Lerp` -90.0 0.0 _newtrack_0)) false false))))

(fn `UserConstructionScript`
  (`InstancedStaticMeshComponent.ClearInstances` (`self.CorpsCasier_ISM`))
  (`InstancedStaticMeshComponent.AddInstance` (`self.CorpsCasier_ISM`) (`KismetMathLibrary.MakeTransform` (43.529775 -35.414615 -1e-06) (struct) (0.03201 0.671341 1.0)) false)
  (`InstancedStaticMeshComponent.AddInstance` (`self.CorpsCasier_ISM`) (`KismetMathLibrary.MakeTransform` (-43.599141 -1.461577 -2e-06) (struct) (0.03201 0.053942 1.0)) false)
  (`InstancedStaticMeshComponent.AddInstance` (`self.CorpsCasier_ISM`) (`KismetMathLibrary.MakeTransform` (0.101245 -35.414615 -52.25128) (struct :`Pitch` -90.0) (0.061708 0.671341 0.900001)) false)
  (`InstancedStaticMeshComponent.AddInstance` (`self.CorpsCasier_ISM`) (`KismetMathLibrary.MakeTransform` (43.529775 -1.461577 -1e-06) (struct) (0.03201 0.053942 1.0)) false)
  (`InstancedStaticMeshComponent.AddInstance` (`self.CorpsCasier_ISM`) (`KismetMathLibrary.MakeTransform` (0.101245 -1.461577 52.014156) (struct :`Pitch` -90.0) (0.061708 0.053942 0.900001)) false)
  (`InstancedStaticMeshComponent.AddInstance` (`self.CorpsCasier_ISM`) (`KismetMathLibrary.MakeTransform` (0.101245 -57.76217 5.479599) (struct :`Pitch` -1e-06 :`Yaw` -90.0 :`Roll` 90.0) (0.061708 0.971672 0.900001)) false)
  (`InstancedStaticMeshComponent.AddInstance` (`self.CorpsCasier_ISM`) (`KismetMathLibrary.MakeTransform` (0.101245 -1.461577 -52.25128) (struct :`Pitch` -90.0) (0.061708 0.053942 0.900001)) false))